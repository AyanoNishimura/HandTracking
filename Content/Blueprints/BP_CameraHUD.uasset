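; BP_CameraHUD is a HUD that starts an Intel RealSense camera and draws its hand-tracking result on screen.
; BeginPlay gets the RealSense context, finds the level's BP_CameraInspector, configures depth, infrared and color streams to matching HD modes with point cloud off, then starts it.
; Each DrawHUD passes the inspector's color texture through a HandTracking call and draws the returned texture.
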(event `self.ReceiveBeginPlay`
  (`self.InitContext`)
  (`self.initInspector`)
  (`self.SetStreamConfiguration`)
  (`self.RunCamera`))

(event `self.ReceiveDrawHUD`
  (params (SizeX :type Integer) (SizeY :type Integer))
  (bind _returnvalue (`TrackingUtils.HandTracking` (`RealSenseInspector.ColorTexture` (`self.RSInspector`))))
  (`self.DrawTextureSimple` _returnvalue))

(fn `InitContext`
  (returns (Context :type "RealSenseContext Object Reference"))
  (`/Engine/EditorBlueprintResources/StandardMacros.IsValid` (`self.RSContext`)
    (:`Is Valid`
      _)
    (:`Is Not Valid`
      (bind _returnvalue (`RealSenseContext.GetRealSense`))
      (set `self.RSContext` _returnvalue)))
  (return (`self.RSContext`)))

(fn `initInspector`
  (`/Engine/EditorBlueprintResources/StandardMacros.IsValid` (`self.RSInspector`)
    (:`Is Not Valid`
      (bind _outactors (`GameplayStatics.GetAllActorsOfClass` "/Game/Blueprints/BP_CameraInspector.BP_CameraInspector_C"))
      (set `self.RSInspector` (`|GetArrayItem` _outactors)))))

(fn `RunCamera`
  (`RealSenseInspector.Start` (`self.RSInspector`)))

(fn `SetStreamConfiguration`
  (bind _realsensestreammode (make `RealSenseStreamMode` 1280 720))
  (bind _rsinspector (`self.RSInspector`))
  (set `RealSenseInspector.DepthConfig` _realsensestreammode _rsinspector)
  (set `RealSenseInspector.InfraredConfig` _realsensestreammode _rsinspector)
  (set `RealSenseInspector.ColorConfig` _realsensestreammode _rsinspector)
  (set `RealSenseInspector.bEnablePcl` false _rsinspector))

(fn `UserConstructionScript`)